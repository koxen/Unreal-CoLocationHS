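; Lobby player controller that runs platform account checks when play begins and reports the results as debug prints.
; After the parent BeginPlay, a sequence starts an entitlement verification that prints success or failure, then checks login status.
; When logged in, it fetches the user profile and prints the profile name.
; Failed checks only print a message, with no further handling.
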(event EventBeginPlay
  (bind (_profile _returnvalue) (Class|OculusXRFunctionLibrary|GetUserProfile))
  (|CallParentFunction)
  (Utilities|FlowControl|Sequence
    (:then_0
      (|VerifyEntitlement
        (:OnSuccess
          (Development|PrintString "ENTITLEMENT CHECK: SUCCESS" true true "(R=0.119021,G=1.000000,B=0.000000,A=1.000000)" 5.0))
        (:OnFailure
          (Development|PrintString "ENTITLEMENT CHECK: FAILURE" true true "(R=1.000000,G=0.000000,B=0.000000,A=1.000000)" 5.0))))
    (:then_1
      (if (Class|KismetSystemLibrary|IsLoggedin self)
        (Development|PrintString "LOGIN CHECK: SUCCESS" true true "(R=0.119021,G=1.000000,B=0.000000,A=1.000000)" 5.0)
        (if _returnvalue
          (Development|PrintString "USER PROFILE CHECK: SUCCESS" true true "(R=0.119021,G=1.000000,B=0.000000,A=1.000000)" 5.0)
          (Development|PrintString (.Name (Utilities|Struct|BreakOculusXRHmdUserProfile _profile)) true true "(R=0.119021,G=1.000000,B=0.000000,A=1.000000)" 5.0)
          (else
            (Development|PrintString "USER PROFILE CHECK: FAILURE" true true "(R=1.000000,G=0.000000,B=0.000000,A=1.000000)" 5.0)))
        (else
          (Development|PrintString "LOGIN CHECK: FAILURE" true true "(R=1.000000,G=0.000000,B=0.000000,A=1.000000)" 5.0))))))

(fn ConstructionScript)